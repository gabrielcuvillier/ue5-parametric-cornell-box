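; Blueprint function library of helpers for building a parametric Cornell box: its walls, emissive panel and rect light.
; Wall helpers derive scale and position from normal axis and dimensions, and color each material slot by wall side through dynamic material instances, reused when already matching.
; Light helpers switch material, visibility, orientation and barn doors per light type, with an area-based factor equating emissive surface intensity to lumens.
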(fn `Compute Wall Dimension`
  (params (Dimension :type "/Game/ParametricCornellBox/Blueprints/ECornellBoxAxis Enum" :default "NewEnumerator0") (`Normal Axis` :type "/Game/ParametricCornellBox/Blueprints/ECornellBoxAxis Enum" :default "NewEnumerator0") (`Reverse Direction` :type Boolean) (Depth :type "Float (double-precision)") (Width :type "Float (double-precision)") (Thickness :type "Float (double-precision)") (`Extra Width` :type Boolean) (`Extra Height` :type Boolean))
  (returns (Value :type "Float (double-precision)"))
  (switch `/Game/ParametricCornellBox/Blueprints/ECornellBoxAxis` `Normal Axis`
    (:`NewEnumerator0`
      (switch `/Game/ParametricCornellBox/Blueprints/ECornellBoxAxis` Dimension
        (:`NewEnumerator0`
          _)
        (:`NewEnumerator1`
          (return (`self.Evaluate Wall Extra Length` Width Thickness `Extra Width`)))
        (:`NewEnumerator2`
          (return (`self.Evaluate Wall Extra Length` Depth Thickness `Extra Height`)))))
    (:`NewEnumerator1`
      (switch `/Game/ParametricCornellBox/Blueprints/ECornellBoxAxis` Dimension
        (:`NewEnumerator0`
          (return (`self.Evaluate Wall Extra Length` Width Thickness `Extra Width`)))
        (:`NewEnumerator1`
          _)
        (:`NewEnumerator2`
          (return (`self.Evaluate Wall Extra Length` Depth Thickness `Extra Height`)))))
    (:`NewEnumerator2`
      (switch `/Game/ParametricCornellBox/Blueprints/ECornellBoxAxis` Dimension
        (:`NewEnumerator0`
          (return (`self.Evaluate Wall Extra Length` Depth Thickness `Extra Height`)))
        (:`NewEnumerator1`
          (return (`self.Evaluate Wall Extra Length` Width Thickness `Extra Width`)))
        (:`NewEnumerator2`
          _))))
  (return Thickness))

(fn `Compute Wall Position`
  (params (`Normal Axis` :type "/Game/ParametricCornellBox/Blueprints/ECornellBoxAxis Enum" :default "NewEnumerator0") (`Reverse Direction` :type Boolean) (Height :type "Float (double-precision)") (Thickness :type "Float (double-precision)"))
  (returns (Value :type "Vector Structure"))
  (return (* (* (`self.Evaluate Axis Direction` `Normal Axis` `Reverse Direction`) -1.0) (/ (+ Height Thickness) 2.0))))

(fn `Create Dynamic Material Instance`
  (params (`Source Material` :type "MaterialInterface Object Reference") (`Target Material` :type "MaterialInterface Object Reference") (`Material Index` :type Integer) (`Primitive Component` :type "PrimitiveComponent Object Reference"))
  (returns (`Material Instance Dynamic` :type "MaterialInstanceDynamic Object Reference"))
  (`/Engine/EditorBlueprintResources/StandardMacros.IsValid` `Source Material`
    (:`Is Valid`
      (bind _returnvalue (`MaterialInterface.GetBaseMaterial` `Source Material`))
      (if (== _returnvalue `Target Material`)
        (bind _asmaterial_instance_dynamic (cast `MaterialInstanceDynamic` `Source Material`)
          (:`then`
            (return _asmaterial_instance_dynamic))
          (:`CastFailed`
            _))))
    (:`Is Not Valid`
      _))
  (bind _returnvalue_2 (`PrimitiveComponent.CreateDynamicMaterialInstance` `Primitive Component` `Material Index` `Target Material` "None"))
  (return _returnvalue_2))

(fn `Evaluate Axis Direction`
  (params (Axis :type "/Game/ParametricCornellBox/Blueprints/ECornellBoxAxis Enum" :default "NewEnumerator0") (`Reverse Direction` :type Boolean))
  (returns (Value :type "Vector Structure"))
  (return (* (select `/Game/ParametricCornellBox/Blueprints/ECornellBoxAxis` Axis :`NewEnumerator0` (1.0 0.0 0.0) :`NewEnumerator1` (0.0 1.0 0.0) :`NewEnumerator2` (0.0 0.0 1.0) :!type "Vector Structure") (select `bool` `Reverse Direction` :`false` 1.0 :`true` -1.0 :!type "Float (single-precision)"))))

(fn `Evaluate Wall Extra Length`
  (params (Dimension :type "Float (double-precision)") (`Extra Length` :type "Float (double-precision)") (`Is Extra` :type Boolean))
  (returns (Value :type "Float (double-precision)"))
  (return (select `bool` `Is Extra` :`false` Dimension :`true` (+ Dimension (* `Extra Length` 2.0)))))

(fn `Material Index to Wall Side`
  (params (`Material Index` :type Integer))
  (returns (Side :type "/Game/ParametricCornellBox/Blueprints/ECornellBoxSide Enum"))
  (return (select `int` `Material Index` :`0` "NewEnumerator5" :`1` "NewEnumerator4" :`2` "NewEnumerator2" :`3` "NewEnumerator3" :`4` "NewEnumerator0" :`5` "NewEnumerator1" :!type "/Game/ParametricCornellBox/Blueprints/ECornellBoxSide Enum")))

(fn `Rotator Sum`
  (params (A :type "Rotator Structure") (B :type "Rotator Structure"))
  (returns (Rotator :type "Rotator Structure"))
  (return (`KismetMathLibrary.MakeRotator` (+ A_Roll B_Roll) (+ A_Pitch B_Pitch) (+ A_Yaw B_Yaw))))

(fn `Setup Emissive Mesh Component`
  (params (`Mesh Component` :type "MeshComponent Object Reference") (`Light Type` :type "/Game/ParametricCornellBox/Blueprints/ECornellBoxLightType Enum" :default "NewEnumerator0") (`Light Color` :type "Color Structure") (`Light Intensity` :type "Float (double-precision)") (`Light Width` :type "Float (double-precision)") (`Light Height` :type "Float (double-precision)") (Visible :type Boolean) (`3D Scale` :type "Vector Structure") (`Unit Length` :type "Float (double-precision)" :default 100.0))
  (returns (`Output Mesh Component` :type "MeshComponent Object Reference"))
  (bind (_x _y _z) (`KismetMathLibrary.BreakVector3f` `3D Scale`))
  (`SceneComponent.SetRelativeScale3D` `Mesh Component` (`KismetMathLibrary.MakeVector` 1.0 (/ `Light Width` `Unit Length`) (/ (* (/ `Light Height` `Unit Length`) _x) _z)))
  (bind _material_instance_dynamic (`self.Create Dynamic Material Instance` (`PrimitiveComponent.GetMaterial` `Mesh Component` 0) (select `/Game/ParametricCornellBox/Blueprints/ECornellBoxLightType` `Light Type` :`NewEnumerator0` "/Game/ParametricCornellBox/Materials/M_CornellBoxPureWhite.M_CornellBoxPureWhite" :`NewEnumerator1` "/Game/ParametricCornellBox/Materials/M_CornellBoxEmissiveNoCast.M_CornellBoxEmissiveNoCast" :`NewEnumerator2` "/Game/ParametricCornellBox/Materials/M_CornellBoxEmissive.M_CornellBoxEmissive" :`NewEnumerator3` "/Game/ParametricCornellBox/Materials/M_CornellBoxPureWhite.M_CornellBoxPureWhite" :`NewEnumerator4` "/Game/ParametricCornellBox/Materials/M_CornellBoxEmissiveNoCast.M_CornellBoxEmissiveNoCast" :!type "MaterialInterface Object Reference") 0 `Mesh Component`))
  (`MaterialInstanceDynamic.SetScalarParameterValue` _material_instance_dynamic "Intensity" (* (select `/Game/ParametricCornellBox/Blueprints/ECornellBoxLightType` `Light Type` :`NewEnumerator1` 1.0 :`NewEnumerator2` `Light Intensity` :`NewEnumerator4` 1.0) (select `/Game/ParametricCornellBox/Blueprints/ECornellBoxLightType` `Light Type` :`NewEnumerator1` 1.0 :`NewEnumerator2` (/ 6290.0 (* `Light Width` `Light Height`)) :`NewEnumerator3` 1.0 :`NewEnumerator4` 1.0)))
  (`MaterialInstanceDynamic.SetVectorParameterValue` _material_instance_dynamic "Color" (`KismetMathLibrary.Conv_ColorToLinearColor` `Light Color`))
  (`PrimitiveComponent.SetEmissiveLightSource` `Mesh Component` (select `/Game/ParametricCornellBox/Blueprints/ECornellBoxLightType` `Light Type` :`NewEnumerator2` true))
  (`PrimitiveComponent.SetCastShadow` `Mesh Component` (select `/Game/ParametricCornellBox/Blueprints/ECornellBoxLightType` `Light Type` :`NewEnumerator3` true))
  (`SceneComponent.SetVisibility` `Mesh Component` (select `/Game/ParametricCornellBox/Blueprints/ECornellBoxLightType` `Light Type` :`NewEnumerator1` Visible :`NewEnumerator2` true :`NewEnumerator3` true :`NewEnumerator4` Visible) false)
  (`PrimitiveComponent.SetVisibleInRayTracing` `Mesh Component` true)
  (return null))

(fn `Setup Rect Light Component`
  (params (`Rect Light Component` :type "RectLightComponent Object Reference") (`Light Type` :type "/Game/ParametricCornellBox/Blueprints/ECornellBoxLightType Enum" :default "NewEnumerator0") (`Light Color` :type "Color Structure") (`Light Intensity` :type "Float (double-precision)") (`Light Width` :type "Float (double-precision)") (`Light Height` :type "Float (double-precision)") (`Light Attenuation Radius` :type "Float (double-precision)") (`Light Depth` :type "Float (double-precision)") (`3D Scale` :type "Vector Structure"))
  (returns (`Output Rect Light Component` :type "RectLightComponent Object Reference"))
  (locals (`Reflected Light Offset` :type "Float (double-precision)" :default 10.0))
  (bind (_x _y _z) (`KismetMathLibrary.BreakVector3f` `3D Scale`))
  (`SceneComponent.K2_SetRelativeLocation` `Rect Light Component` (0.25 0.0 0.0) false false)
  (`SceneComponent.SetVisibility` `Rect Light Component` (select `/Game/ParametricCornellBox/Blueprints/ECornellBoxLightType` `Light Type` :`NewEnumerator1` true :`NewEnumerator3` true :`NewEnumerator4` true) false)
  (`SceneComponent.K2_SetRelativeRotation` `Rect Light Component` (`KismetMathLibrary.MakeRotator` 0.0 (select `/Game/ParametricCornellBox/Blueprints/ECornellBoxLightType` `Light Type` :`NewEnumerator3` 180.0)) false false)
  (`LocalLightComponent.SetAttenuationRadius` `Rect Light Component` (* `Light Attenuation Radius` (/ (`KismetMathLibrary.VSize` `3D Scale`) (`KismetMathLibrary.VSize` (1.0 1.0 1.0)))))
  (`RectLightComponent.SetSourceWidth` `Rect Light Component` (* `Light Width` _y))
  (`RectLightComponent.SetSourceHeight` `Rect Light Component` (* _x `Light Height`))
  (`LightComponent.SetIntensity` `Rect Light Component` `Light Intensity`)
  (`LightComponent.SetLightColor` `Rect Light Component` (`KismetMathLibrary.Conv_ColorToLinearColor` `Light Color`) true)
  (`RectLightComponent.SetBarnDoorAngle` `Rect Light Component` 0.0)
  (`RectLightComponent.SetBarnDoorLength` `Rect Light Component` (select `/Game/ParametricCornellBox/Blueprints/ECornellBoxLightType` `Light Type` :`NewEnumerator3` 0.5 :`NewEnumerator4` (* _z `Light Depth`) :!type "Float (single-precision)"))
  (`LightComponentBase.SetCastShadows` `Rect Light Component` true)
  (`LightComponentBase.SetCastRaytracedShadows` `Rect Light Component` "UseProjectSetting")
  (`LightComponentBase.SetAffectGlobalIllumination` `Rect Light Component` true)
  (`LightComponentBase.SetAffectReflection` `Rect Light Component` true)
  (return `Rect Light Component`))

(fn `Setup Wall Mesh Component Geometry`
  (params (`Mesh Component` :type "MeshComponent Object Reference") (`Normal Axis` :type "/Game/ParametricCornellBox/Blueprints/ECornellBoxAxis Enum" :default "NewEnumerator0") (`Reverse Direction` :type Boolean) (Depth :type "Float (single-precision)") (Width :type "Float (single-precision)") (Height :type "Float (double-precision)") (Thickness :type "Float (double-precision)") (`Extra Width` :type Boolean) (`Extra Height` :type Boolean) (`Unit Length` :type "Float (double-precision)" :default 100.0))
  (returns (`Output Mesh` :type "MeshComponent Object Reference"))
  (locals (`Dimension X` :type "Float (double-precision)") (`Dimension Y` :type "Float (double-precision)") (`Dimension Z` :type "Float (double-precision)"))
  (bind _enumvalue (foreach `/Game/ParametricCornellBox/Blueprints/ECornellBoxAxis` false)
    (:`LoopBody`
      (switch `/Game/ParametricCornellBox/Blueprints/ECornellBoxAxis` _enumvalue
        (:`NewEnumerator0`
          (bind _value (`self.Compute Wall Dimension` _enumvalue `Normal Axis` `Reverse Direction` Depth Width Thickness `Extra Width` `Extra Height`))
          (bind _output_get (set `local.Dimension X` _value)))
        (:`NewEnumerator1`
          (bind _output_get_2 (set `local.Dimension Y` _value)))
        (:`NewEnumerator2`
          (bind _output_get_3 (set `local.Dimension Z` _value)))))
    (:`then`
      (`SceneComponent.SetRelativeScale3D` `Mesh Component` (`KismetMathLibrary.MakeVector` (/ _output_get `Unit Length`) (/ _output_get_2 `Unit Length`) (/ _output_get_3 `Unit Length`)))
      (`SceneComponent.K2_SetRelativeLocation` `Mesh Component` (`self.Compute Wall Position` `Normal Axis` `Reverse Direction` Height Thickness) false false)
      (return `Mesh Component`))))

(fn `Setup Wall Mesh Component Material`
  (params (`Mesh Component` :type "MeshComponent Object Reference") (Metallic :type "Float (double-precision)") (Specular :type "Float (double-precision)") (Roughness :type "Float (double-precision)") (`Neutral Color` :type "Color Structure") (`Left Color` :type "Color Structure") (`Right Color` :type "Color Structure") (`External Color` :type "Color Structure") (Wall :type "/Game/ParametricCornellBox/Blueprints/ECornellBoxSide Enum" :default "NewEnumerator0"))
  (returns (`Output Mesh Component` :type "MeshComponent Object Reference"))
  (locals (NewLocalVar :type "AbcConversionSettings Structure"))
  (for (_array_element _array_index) (`MeshComponent.GetMaterials` `Mesh Component`)
    (bind _material_instance_dynamic (`self.Create Dynamic Material Instance` _array_element "/Game/ParametricCornellBox/Materials/M_CornellBoxWhiteWall.M_CornellBoxWhiteWall" _array_index `Mesh Component`))
    (`MaterialInstanceDynamic.SetScalarParameterValue` _material_instance_dynamic "Metallic" Metallic)
    (`MaterialInstanceDynamic.SetScalarParameterValue` _material_instance_dynamic "Specular" Specular)
    (`MaterialInstanceDynamic.SetScalarParameterValue` _material_instance_dynamic "Roughness" Roughness)
    (bind _side (`self.Material Index to Wall Side` _array_index))
    (`MaterialInstanceDynamic.SetVectorParameterValue` _material_instance_dynamic "Color" (`KismetMathLibrary.Conv_ColorToLinearColor` (select `/Game/ParametricCornellBox/Blueprints/ECornellBoxSide` Wall :`NewEnumerator0` (select `/Game/ParametricCornellBox/Blueprints/ECornellBoxSide` _side :`NewEnumerator0` `External Color` :`NewEnumerator1` `Neutral Color` :`NewEnumerator2` `External Color` :`NewEnumerator3` `External Color` :`NewEnumerator4` `External Color` :`NewEnumerator5` `External Color`) :`NewEnumerator1` (select `/Game/ParametricCornellBox/Blueprints/ECornellBoxSide` _side :`NewEnumerator0` `Neutral Color` :`NewEnumerator1` `External Color` :`NewEnumerator2` `External Color` :`NewEnumerator3` `External Color` :`NewEnumerator4` `External Color` :`NewEnumerator5` `External Color`) :`NewEnumerator2` (select `/Game/ParametricCornellBox/Blueprints/ECornellBoxSide` _side :`NewEnumerator0` `External Color` :`NewEnumerator1` `External Color` :`NewEnumerator2` `External Color` :`NewEnumerator3` `Left Color` :`NewEnumerator4` `External Color` :`NewEnumerator5` `External Color`) :`NewEnumerator3` (select `/Game/ParametricCornellBox/Blueprints/ECornellBoxSide` _side :`NewEnumerator0` `External Color` :`NewEnumerator1` `External Color` :`NewEnumerator2` `Right Color` :`NewEnumerator3` `External Color` :`NewEnumerator4` `External Color` :`NewEnumerator5` `External Color`) :`NewEnumerator4` (select `/Game/ParametricCornellBox/Blueprints/ECornellBoxSide` _side :`NewEnumerator0` `External Color` :`NewEnumerator1` `External Color` :`NewEnumerator2` `External Color` :`NewEnumerator3` `External Color` :`NewEnumerator4` `External Color` :`NewEnumerator5` `Neutral Color`) :`NewEnumerator5` (select `/Game/ParametricCornellBox/Blueprints/ECornellBoxSide` _side :`NewEnumerator0` `External Color` :`NewEnumerator1` `External Color` :`NewEnumerator2` `External Color` :`NewEnumerator3` `External Color` :`NewEnumerator4` `Neutral Color`)))))
  (return `Mesh Component`))

(fn `Switch Vector 2D`
  (params (In :type "Vector2D Structure") (Switch :type Boolean))
  (returns (Out :type "Vector2D Structure"))
  (return (`KismetMathLibrary.MakeVector2D` (select `bool` Switch :`false` In_X :`true` In_Y) (select `bool` Switch :`false` In_Y :`true` In_X))))

(fn `Toggle Scene Component (Destroy)`
  (params (`Scene Component` :type "SceneComponent Object Reference") (Visible :type Boolean))
  (if (not Visible)
    (`ActorComponent.K2_DestroyComponent` `Scene Component`)))