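; Parametric Cornell Box actor that rebuilds its walls, lighting and contents in the construction script.
; Wall specification and axis maps drive each visible wall's size, orientation, inside/outside colors and material.
; The light rig orients to a chosen side, optionally substituting or disabling light types that fail under static lighting.
; Content switches between empty, classic cubes, sample sphere, calibration spheres or a user mesh, toggling off unused components.
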(fn `Get Box Color Value`
  (params (Color :type "/Game/ParametricCornellBox/Blueprints/Internal/E_CornellBox_Color Enum" :default "NewEnumerator0"))
  (returns (Value :type "Color Structure"))
  (return (select `/Game/ParametricCornellBox/Blueprints/Internal/E_CornellBox_Color` Color :`NewEnumerator0` (`self.Neutral Color`) :`NewEnumerator1` (`self.Left Color`) :`NewEnumerator2` (`self.Right Color`) :`NewEnumerator3` (`self.External Color`))))

(fn `Get Box Dimension Value`
  (params (Dimension :type "/Game/ParametricCornellBox/Blueprints/Internal/E_CornellBox_Dimension Enum" :default "NewEnumerator0"))
  (returns (Value :type "Float (double-precision)"))
  (return (select `/Game/ParametricCornellBox/Blueprints/Internal/E_CornellBox_Dimension` Dimension :`NewEnumerator0` (`self.Box Depth (X)`) :`NewEnumerator1` (`self.Box Width (Y)`) :`NewEnumerator2` (`self.Box Height (Z)`) :`NewEnumerator4` (`self.Wall Thickness`))))

(fn `Get Box Wall Mesh Component`
  (params (Side :type "/Game/ParametricCornellBox/Blueprints/Internal/E_CornellBox_Side Enum" :default "NewEnumerator0"))
  (returns (`Mesh Component` :type "MeshComponent Object Reference"))
  (return (select `/Game/ParametricCornellBox/Blueprints/Internal/E_CornellBox_Side` Side :`NewEnumerator0` (`self.Front Wall`) :`NewEnumerator1` (`self.Back Wall`) :`NewEnumerator2` (`self.Left Wall`) :`NewEnumerator3` (`self.Right Wall`) :`NewEnumerator4` (`self.Top Wall`) :`NewEnumerator5` (`self.Bottom Wall`))))

(fn `Update All`
  (`self.Update Geometry`)
  (`self.Update Lighting`)
  (`self.Update Content`))

(fn `Update Content`
  (bind _content_type (`self.Content Type`))
  (bind _content (`self.Content`))
  (bind _content_scale (`self.Content Scale`))
  (bind _tall_cube (`self.Tall Cube`))
  (bind _content_type_2 (`self.Content Type`))
  (bind _content_mobility (`self.Content Mobility`))
  (bind _small_cube (`self.Small Cube`))
  (bind _content_mobility_2 (`self.Content Mobility`))
  (bind _sample_sphere (`self.Sample Sphere`))
  (bind _black_sphere (`self.Black Sphere`))
  (bind _chrome_sphere (`self.Chrome Sphere`))
  (bind _white_sphere (`self.White Sphere`))
  (bind _user_static_mesh (`self.User Static Mesh`))
  (bind _returnvalue (`|EnumEquality` _content_type "NewEnumerator1"))
  (bind _returnvalue_2 (select `/Game/ParametricCornellBox/Blueprints/Internal/E_CornellBox_ContentType` _content_type_2 :`NewEnumerator4` true))
  (bind _returnvalue_3 (select `/Game/ParametricCornellBox/Blueprints/Internal/E_CornellBox_ContentType` _content_type_2 :`NewEnumerator1` true))
  (`|ExecutionSequence`
    (:`then_0`
      ;[1 1 1] Setup Transformation
      (`SceneComponent.K2_SetRelativeRotation` _content (`KismetMathLibrary.MakeRotator` 0.0 0.0 (`self.Content Rotation`)) false false)
      (`SceneComponent.SetRelativeScale3D` _content (`KismetMathLibrary.MakeVector` _content_scale _content_scale _content_scale))
      (`SceneComponent.K2_SetRelativeLocation` _content (`KismetMathLibrary.MakeVector` 0.0 0.0 (`self.Content Height`)) false false))
    (:`then_1`
      ;[1 1 1] Setup Static Mesh
      (if (`|EnumEquality` _content_type "NewEnumerator3")
        (`StaticMeshComponent.SetStaticMesh` _user_static_mesh (`self.Content User Mesh`))
        (`SceneComponent.SetMobility` _user_static_mesh (`self.Content Mobility`))))
    (:`then_2`
      ;[1 1 1] Setup Classic Cubes and Sample Sphere
      (if _returnvalue
        (`PrimitiveComponent.SetMaterial` _tall_cube 0 (`self.Tall Cube Material`))
        (`SceneComponent.SetMobility` _tall_cube _content_mobility)))
    (:`then_3`
      (if _returnvalue
        (`PrimitiveComponent.SetMaterial` _small_cube 0 (`self.Small Cube Material`))
        (`SceneComponent.SetMobility` _small_cube _content_mobility)))
    (:`then_4`
      (if (`|EnumEquality` _content_type "NewEnumerator2")
        (`PrimitiveComponent.SetMaterial` _sample_sphere 0 (`self.Sphere Material`))
        (`SceneComponent.SetMobility` _sample_sphere _content_mobility)))
    (:`then_5`
      ;[1 1 1] Setup Calibration Spheres
      (if (`|EnumEquality` _content_type "NewEnumerator4")
        (`|ExecutionSequence`
          (:`then_0`
            (`PrimitiveComponent.SetMaterial` _black_sphere 0 "/Game/ParametricCornellBox/Materials/MI_Black.MI_Black")
            (`PrimitiveComponent.SetMaterial` _chrome_sphere 0 "/Game/ParametricCornellBox/Materials/MI_Chrome.MI_Chrome")
            (`PrimitiveComponent.SetMaterial` _white_sphere 0 "/Game/ParametricCornellBox/Materials/MI_White.MI_White"))
          (:`then_1`
            (`SceneComponent.SetMobility` _black_sphere _content_mobility_2)
            (`SceneComponent.SetMobility` _chrome_sphere _content_mobility_2)
            (`SceneComponent.SetMobility` _white_sphere _content_mobility_2)))))
    (:`then_6`
      ;[1 1 1] Destroy what is not used
      (`/Game/ParametricCornellBox/Blueprints/Internal/BPFL_CornellBox_Utils.Toggle Scene Component` (`self.Tall Cube`) _returnvalue_3)
      (`/Game/ParametricCornellBox/Blueprints/Internal/BPFL_CornellBox_Utils.Toggle Scene Component` (`self.Small Cube`) _returnvalue_3)
      (`/Game/ParametricCornellBox/Blueprints/Internal/BPFL_CornellBox_Utils.Toggle Scene Component` (`self.Sample Sphere`) (select `/Game/ParametricCornellBox/Blueprints/Internal/E_CornellBox_ContentType` _content_type_2 :`NewEnumerator2` true))
      (`/Game/ParametricCornellBox/Blueprints/Internal/BPFL_CornellBox_Utils.Toggle Scene Component` (`self.User Static Mesh`) (select `/Game/ParametricCornellBox/Blueprints/Internal/E_CornellBox_ContentType` _content_type_2 :`NewEnumerator3` true))
      (`/Game/ParametricCornellBox/Blueprints/Internal/BPFL_CornellBox_Utils.Toggle Scene Component` (`self.Black Sphere`) _returnvalue_2)
      (`/Game/ParametricCornellBox/Blueprints/Internal/BPFL_CornellBox_Utils.Toggle Scene Component` (`self.Chrome Sphere`) _returnvalue_2)
      (`/Game/ParametricCornellBox/Blueprints/Internal/BPFL_CornellBox_Utils.Toggle Scene Component` (`self.White Sphere`) _returnvalue_2))))

(fn `Update Geometry`
  (bind _box_wall_specification (`self.Box Wall Specification`))
  ;[1 1 1] Move Geometry node by half Box Height
  (`SceneComponent.K2_SetRelativeLocation` (`self.Geometry`) (`KismetMathLibrary.MakeVector` 0.0 0.0 (/ (`self.Box Height (Z)`) 2.0)) false false)
  ;[1 1 1] For Each Wall Specification
  (bind _keys (`BlueprintMapLibrary.Map_Keys` _box_wall_specification))
  (for _array_element _keys
    (bind (_value _returnvalue) (`BlueprintMapLibrary.Map_Find` _box_wall_specification _array_element))
    (if _returnvalue
      (bind (_value_2 _returnvalue_2) (`BlueprintMapLibrary.Map_Find` (`self.Wall Visibilities`) _array_element))
      (if (and _value_2 _returnvalue_2)
        (bind _mesh_component (`self.Get Box Wall Mesh Component` _array_element))
        (bind ((`NormalAxis_158_03BB1C2849F0FC3E441940A5CEE3BC9A` _normalaxis) (`ReverseDirection_160_28F05AC14693334E5187E8A4DE7FDD6C` _reversedirection) (`ExtraWidth_155_8FF2A5D2409666FD5211E1840A96A7B9` _extrawidth) (`ExtraHeight_157_DA36CDDD4D38732E1F7F35BD06E9DFDA` _extraheight) (`WallSidesLocation_172_91B6D93A45FDEC80706111B9A82303E4` _wallsideslocation) (`InsideColor_176_B620076B4F905D3407E02E83C3F6DBCD` _insidecolor) (`OutsideColor_178_47A06C564F3435AC8BB650B180488402` _outsidecolor)) (break `/Game/ParametricCornellBox/Blueprints/Internal/F_CornellBox_WallSpecification` _value))
        ;[1 1 1] Retrieval of Box data according to Wall specification
        ;;[1 1 1] Setup the Mesh Component Material
        (bind _output_mesh_component (`/Game/ParametricCornellBox/Blueprints/Internal/BPFL_CornellBox_Utils.Setup Wall Mesh Component Material` _mesh_component (`self.Metalness`) (`self.Specularity`) (`self.Roughness`) _wallsideslocation (`self.Get Box Color Value` _insidecolor) (`self.Get Box Color Value` _outsidecolor)))
        (bind (_value_3 _returnvalue_3) (`BlueprintMapLibrary.Map_Find` (`self.Axis Wall Parameters Specification`) _normalaxis))
        (if _returnvalue_3
          ;[1 1 1] Setup Wall Mesh Geometry
          (bind _output_mesh (`/Game/ParametricCornellBox/Blueprints/Internal/BPFL_CornellBox_Utils.Setup Wall Mesh Component Geometry` _output_mesh_component _normalaxis _reversedirection (`self.Get Box Dimension Value` (break `/Game/ParametricCornellBox/Blueprints/Internal/F_CornellBox_WallParameters` _value_3)) (`self.Get Box Dimension Value` (`.WallWidth_2_DB38E35443B05D9763FE0B9DD68F17B9` (break `/Game/ParametricCornellBox/Blueprints/Internal/F_CornellBox_WallParameters` _value_3))) (`self.Get Box Dimension Value` (`.WallHeight_12_5165DB824CDF33FCFAC6D3A8928DE44E` (break `/Game/ParametricCornellBox/Blueprints/Internal/F_CornellBox_WallParameters` _value_3))) (`self.Wall Thickness`) _extrawidth _extraheight))
          (`SceneComponent.SetMobility` _output_mesh (`self.Geometry Mobility`)))
        (else
          (`/Game/ParametricCornellBox/Blueprints/Internal/BPFL_CornellBox_Utils.Toggle Scene Component` _mesh_component))))))

(fn `Update Lighting`
  (locals (LocalLightDepth :type "Float (double-precision)") (LocalLightType :type "/Game/ParametricCornellBox/Blueprints/Internal/E_CornellBox_LightType Enum"))
  (bind _lighting_system (`self.Lighting System`))
  (bind _source_system (`self.Source System`))
  (bind _light_height (`self.Light Height`))
  (bind _light_color (`self.Light Color`))
  (bind _light_mobility (`self.Light Mobility`))
  (bind _light_intensity__lm_ (`self.Light Intensity (lm)`))
  (bind _light_width (`self.Light Width`))
  (bind (_value _returnvalue) (`BlueprintMapLibrary.Map_Find` (`self.Box Wall Specification`) (`self.Light Side`)))
  (bind (_x _y) (`KismetMathLibrary.BreakVector2D` (`self.Light Position`)))
  (bind _relativescale3d (`SceneComponent.RelativeScale3D` (`self.DefaultSceneRoot`)))
  (bind _returnvalue_2 (not (`|EnumEquality` (`self.Light Mobility`) "Movable")))
  (bind (_value_2 _returnvalue_3) (`BlueprintMapLibrary.Map_Find` (`self.Axis Wall Parameters Specification`) (break `/Game/ParametricCornellBox/Blueprints/Internal/F_CornellBox_WallSpecification` _value)))
  (bind (_out_x _out_y) (`KismetMathLibrary.BreakVector2D` (`/Game/ParametricCornellBox/Blueprints/Internal/BPFL_CornellBox_Utils.Switch Vector 2D` (`KismetMathLibrary.MakeVector2D` _x (select `bool` (`.RevertLightPositionYOffset_164_C63E8B5E464329AA900DF7BFB7D0A0E3` (break `/Game/ParametricCornellBox/Blueprints/Internal/F_CornellBox_WallSpecification` _value)) :`false` _y :`true` (* _y -1.0))) (`.SwitchLightPositionOffset_141_734779F9495D1C96BBB036A243F58DDF` (break `/Game/ParametricCornellBox/Blueprints/Internal/F_CornellBox_WallSpecification` _value)))))
  (`SceneComponent.SetMobility` (`self.Rect Light`) _light_mobility)
  (`SceneComponent.SetMobility` (`self.Emissive Surface`) _light_mobility)
  ;[1 1 1] Setup Lighting System and Source System Transformations
  (if (and _returnvalue_3 _returnvalue)
    (`SceneComponent.K2_SetRelativeRotation` _lighting_system (`/Game/ParametricCornellBox/Blueprints/Internal/BPFL_CornellBox_Utils.Rotator Sum` (`.LightRotation_138_DC27AE23484FA87932BE04A2B848DA9B` (break `/Game/ParametricCornellBox/Blueprints/Internal/F_CornellBox_WallSpecification` _value)) (`self.Light Rotation Offset`)) false false)
    (`SceneComponent.K2_SetRelativeLocation` _lighting_system (`KismetMathLibrary.MakeVector` 0.0 0.0 (/ (`self.Box Height (Z)`) 2.0)) false false)
    (bind _output_get (set `local.LocalLightDepth` (`self.Get Box Dimension Value` (`.WallHeight_12_5165DB824CDF33FCFAC6D3A8928DE44E` (break `/Game/ParametricCornellBox/Blueprints/Internal/F_CornellBox_WallParameters` _value_2)))))
    (`SceneComponent.K2_SetRelativeLocation` _source_system (`KismetMathLibrary.MakeVector` _out_x _out_y (- (/ _output_get 2.0) (`self.Light Z Offset`))) false false)
    (`SceneComponent.K2_SetRelativeRotation` _source_system (struct :`Pitch` -90.0) false false)
    ;[1 1 1] Setup the Light components
    (bind _output_get_2 (set `local.LocalLightType` (select `/Game/ParametricCornellBox/Blueprints/Internal/E_CornellBox_LightType` (`self.Light Type`) :`NewEnumerator0` "NewEnumerator0" :`NewEnumerator1` "NewEnumerator1" :`NewEnumerator2` (select `bool` (and (`self.Use Reflected Light for Emissive in Static Lighting`) _returnvalue_2) :`false` "NewEnumerator2" :`true` "NewEnumerator3" :!type "/Game/ParametricCornellBox/Blueprints/Internal/E_CornellBox_LightType Enum") :`NewEnumerator3` "NewEnumerator3" :`NewEnumerator4` (select `bool` (and _returnvalue_2 (`self.Disable Directional Light in Static Lighting`)) :`false` "NewEnumerator4" :`true` "NewEnumerator0" :!type "/Game/ParametricCornellBox/Blueprints/Internal/E_CornellBox_LightType Enum"))))
    (`|ExecutionSequence`
      (:`then_0`
        (`/Game/ParametricCornellBox/Blueprints/Internal/BPFL_CornellBox_Utils.Setup Emissive Mesh Component` (`self.Emissive Surface`) _output_get_2 _light_color _light_intensity__lm_ _light_width _light_height (`self.Visible Rect Light Surface`) _relativescale3d))
      (:`then_1`
        (`/Game/ParametricCornellBox/Blueprints/Internal/BPFL_CornellBox_Utils.Setup Rect Light Component` (`self.Rect Light`) _output_get_2 _light_color _light_intensity__lm_ _light_width _light_height (* (`self.Light Attenuation Scale`) (`KismetMathLibrary.FMax` (`self.Box Depth (X)`) (`self.Box Width (Y)`) (* (`self.Box Height (Z)`) 1.5))) _output_get _relativescale3d)))))

(fn `UserConstructionScript`
  (`self.Update All`))