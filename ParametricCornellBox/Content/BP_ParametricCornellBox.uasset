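; Parametric Cornell box actor that rebuilds its walls, area light and sample content in the construction script from exposed dimensions, colors and options.
; Spec maps drive per-wall materials and geometry, with optional hiding of front and top walls.
; A chosen light side orients a rect light and matching emissive surface, with attenuation radius derived from box size.
; A content enum toggles hemicubes, sphere, calibration spheres or a user mesh, including collision and transform.
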(fn `Get Parameter Value`
  (params (Parameter :type "/ParametricCornellBox/Blueprints/ECornellBoxParameter Enum" :default "NewEnumerator0"))
  (returns (Value :type "Float (double-precision)"))
  (return (select `/ParametricCornellBox/Blueprints/ECornellBoxParameter` Parameter :`NewEnumerator0` (`self.Box Depth (X)`) :`NewEnumerator1` (`self.Box Width (Y)`) :`NewEnumerator2` (`self.Box Height (Z)`) :`NewEnumerator4` (`self.Wall Thickness`))))

(fn `Get Wall Mesh Component`
  (params (Wall :type "/ParametricCornellBox/Blueprints/ECornellBoxSide Enum" :default "NewEnumerator0"))
  (returns (Value :type "MeshComponent Object Reference"))
  (return (select `/ParametricCornellBox/Blueprints/ECornellBoxSide` Wall :`NewEnumerator0` (`self.Front Wall`) :`NewEnumerator1` (`self.Back Wall`) :`NewEnumerator2` (`self.Left Wall`) :`NewEnumerator3` (`self.Right Wall`) :`NewEnumerator4` (`self.Top Wall`) :`NewEnumerator5` (`self.Bottom Wall`) :!type "MeshComponent Object Reference")))

(fn `Update Content`
  (bind _content_type (`self.Content Type`))
  (bind _content (`self.Content`))
  (bind _scale (`self.Scale`))
  (bind _sphere (`self.Sphere`))
  (bind _static_mesh (`self.Static Mesh`))
  (bind _returnvalue (select `/ParametricCornellBox/Blueprints/ECornellBoxContentType` _content_type :`NewEnumerator3` true))
  (bind _returnvalue_2 (select `/ParametricCornellBox/Blueprints/ECornellBoxContentType` _content_type :`NewEnumerator4` true))
  (bind _returnvalue_3 (select `/ParametricCornellBox/Blueprints/ECornellBoxContentType` _content_type :`NewEnumerator2` true))
  (bind _returnvalue_4 (select `/ParametricCornellBox/Blueprints/ECornellBoxContentType` _content_type :`NewEnumerator1` true))
  (bind _returnvalue_5 (select `bool` _returnvalue_2 :`false` "NoCollision" :`true` "QueryAndPhysics" :!type "ECollisionEnabled Enum"))
  (bind _returnvalue_6 (select `bool` _returnvalue_4 :`false` "NoCollision" :`true` "QueryAndPhysics" :!type "ECollisionEnabled Enum"))
  (`|ExecutionSequence`
    (:`then_0`
      (`SceneComponent.SetVisibility` (`self.Content`) (select `/ParametricCornellBox/Blueprints/ECornellBoxContentType` _content_type :`NewEnumerator1` true :`NewEnumerator2` true :`NewEnumerator4` true :`NewEnumerator3` true) true)
      (`SceneComponent.SetVisibility` (`self.Hemicubes`) _returnvalue_4 true)
      (`SceneComponent.SetVisibility` _sphere _returnvalue_3 false)
      (`SceneComponent.SetVisibility` _static_mesh _returnvalue false)
      (`SceneComponent.SetVisibility` (`self.Calibration Spheres`) _returnvalue_2 true))
    (:`then_1`
      (`StaticMeshComponent.SetStaticMesh` (`self.Static Mesh`) (`self.User Mesh`)))
    (:`then_2`
      (`PrimitiveComponent.SetCollisionEnabled` (`self.Hemicube 1`) _returnvalue_6)
      (`PrimitiveComponent.SetCollisionEnabled` (`self.Hemicube 2`) _returnvalue_6)
      (`PrimitiveComponent.SetCollisionEnabled` _sphere (select `bool` _returnvalue_3 :`false` "NoCollision" :`true` "QueryAndPhysics" :!type "ECollisionEnabled Enum"))
      (`PrimitiveComponent.SetCollisionEnabled` _static_mesh (select `bool` _returnvalue :`false` "NoCollision" :`true` "QueryAndPhysics" :!type "ECollisionEnabled Enum"))
      (`PrimitiveComponent.SetCollisionEnabled` (`self.Black`) _returnvalue_5)
      (`PrimitiveComponent.SetCollisionEnabled` (`self.Chrome`) _returnvalue_5)
      (`PrimitiveComponent.SetCollisionEnabled` (`self.White`) _returnvalue_5))
    (:`then_3`
      (`SceneComponent.K2_SetRelativeRotation` _content (`KismetMathLibrary.MakeRotator` 0.0 0.0 (`self.Rotation`)) false false)
      (`SceneComponent.SetRelativeScale3D` _content (`KismetMathLibrary.MakeVector` _scale _scale _scale))
      (`SceneComponent.K2_SetRelativeLocation` _content (`KismetMathLibrary.MakeVector` 0.0 0.0 (`self.Height`)) false false))))

(fn `Update Geometry`
  (bind _box_wall_specification (`self.Box Wall Specification`))
  (bind _keys (`BlueprintMapLibrary.Map_Keys` _box_wall_specification))
  (for _array_element _keys
    (bind _returnvalue (`|EnumEquality` _array_element "NewEnumerator0"))
    (bind _returnvalue_2 (`|EnumEquality` _array_element "NewEnumerator4"))
    (bind (_value _returnvalue_3) (`BlueprintMapLibrary.Map_Find` _box_wall_specification _array_element))
    (if (and (or (and (not (`self.Hide Front Wall`)) _returnvalue) (and (not _returnvalue) (not _returnvalue_2)) (and (not (`self.Hide Top Wall`)) _returnvalue_2)) _returnvalue_3)
      (bind _value_2 (`self.Get Wall Mesh Component` _array_element))
      (`/ParametricCornellBox/Blueprints/BPFL_CornellBoxUtils.Setup Wall Mesh Component Material` _value_2 (`self.Metalness`) (`self.Specularity`) (`self.Roughness`) (`self.Neutral Color`) (`self.Left Color`) (`self.Right Color`) (`self.External Color`) _array_element)
      (bind (_axis _reverse _extrawidth _extraheight) (break `/ParametricCornellBox/Blueprints/SCornellBoxWallSpecification` _value))
      (bind (_value_3 _returnvalue_4) (`BlueprintMapLibrary.Map_Find` (`self.Axis Wall Parameters Specification`) _axis))
      (if _returnvalue_4
        (bind _value_4 (`self.Get Parameter Value` (break `/ParametricCornellBox/Blueprints/SCornellBoxWallParameters` _value_3)))
        (bind _value_5 (`self.Get Parameter Value` (`.WallHeight_5_94F7493C4645D46196436591FB3833B2` (break `/ParametricCornellBox/Blueprints/SCornellBoxWallParameters` _value_3))))
        (bind _value_6 (`self.Get Parameter Value` (`.Depth_6_5165DB824CDF33FCFAC6D3A8928DE44E` (break `/ParametricCornellBox/Blueprints/SCornellBoxWallParameters` _value_3))))
        (`/ParametricCornellBox/Blueprints/BPFL_CornellBoxUtils.Setup Wall Mesh Component Geometry` _value_2 _axis _reverse _value_4 _value_5 _value_6 (`self.Wall Thickness`) _extrawidth _extraheight (`self.Box Height (Z)`)))
      (else
        (bind _value_7 (`self.Get Wall Mesh Component` _array_element))
        (`SceneComponent.SetVisibility` _value_7 false false)
        (`PrimitiveComponent.SetCollisionEnabled` _value_7 "NoCollision")))))

(fn `Update Lighting`
  (bind _lighting_system (`self.Lighting System`))
  (bind _source_system (`self.Source System`))
  (bind _light_type (`self.Light Type`))
  (bind _light_height (`self.Light Height`))
  (bind _light_color (`self.Light Color`))
  (bind _light_mobility (`self.Light Mobility`))
  (bind _light_intensity__lm_ (`self.Light Intensity (lm)`))
  (bind _light_width (`self.Light Width`))
  (bind (_value _returnvalue) (`BlueprintMapLibrary.Map_Find` (`self.Light Side Specification`) (`self.Light Side`)))
  (bind _relativescale3d (`SceneComponent.RelativeScale3D` (`self.DefaultSceneRoot`)))
  (bind (_out_x _out_y) (`KismetMathLibrary.BreakVector2D` (`/ParametricCornellBox/Blueprints/BPFL_CornellBoxUtils.Switch Vector 2D` (`self.Light Position Offset`) (`.SwitchLightPositionOffset_14_A4AFBBC943B1BF47E9A86E81B8013B8F` (break `/ParametricCornellBox/Blueprints/SCornellBoxLightSideSpecification` _value)))))
  (`SceneComponent.SetMobility` (`self.Rect Light`) _light_mobility)
  (`SceneComponent.SetMobility` (`self.Emissive Surface`) _light_mobility)
  (if _returnvalue
    (`SceneComponent.K2_SetRelativeRotation` _lighting_system (`/ParametricCornellBox/Blueprints/BPFL_CornellBoxUtils.Rotator Sum` (`.LightRotation_12_A0A0E5194A9A01C0F8C7BD879842E843` (break `/ParametricCornellBox/Blueprints/SCornellBoxLightSideSpecification` _value)) (`self.Light Rotation Offset`)) false false)
    (`SceneComponent.K2_SetRelativeLocation` _lighting_system (`KismetMathLibrary.MakeVector` 0.0 0.0 (/ (`self.Box Height (Z)`) 2.0)) false false)
    (bind _value_2 (`self.Get Parameter Value` (break `/ParametricCornellBox/Blueprints/SCornellBoxLightSideSpecification` _value)))
    (`SceneComponent.K2_SetRelativeLocation` _source_system (`KismetMathLibrary.MakeVector` _out_x _out_y (- (/ _value_2 2.0) (`self.Light Z Offset`))) false false)
    (`SceneComponent.K2_SetRelativeRotation` _source_system (struct :`Pitch` -90.0) false false)
    (`|ExecutionSequence`
      (:`then_0`
        (`/ParametricCornellBox/Blueprints/BPFL_CornellBoxUtils.Setup Emissive Mesh Component` (`self.Emissive Surface`) _light_type _light_color _light_intensity__lm_ _light_width _light_height (`self.Visible Rect Light Surface`) _relativescale3d))
      (:`then_1`
        (`/ParametricCornellBox/Blueprints/BPFL_CornellBoxUtils.Setup Rect Light Component` (`self.Rect Light`) _light_type _light_color _light_intensity__lm_ _light_width _light_height (* (`self.Light Attenuation Scale`) (`KismetMathLibrary.FMax` (`self.Box Depth (X)`) (`self.Box Width (Y)`) (* (`self.Box Height (Z)`) 1.5))) _value_2 _relativescale3d)))))

(fn `UserConstructionScript`
  (`self.Update Geometry`)
  (`self.Update Lighting`)
  (`self.Update Content`))